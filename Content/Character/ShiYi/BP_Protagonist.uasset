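; Player character Blueprint for the protagonist, handling camera control and zoom, movement, sprint, crouch and attack input flags, and opening a UI-only player menu.
; While fire mode is toggled on, Tick draws a dynamic brush material at the normalized actor position into a render target, a clearable grass-burn mask.
; A timed invisibility skill swaps mesh materials and animates Alpha through a timeline.
; The 3D UI render-target and hair-color setup is never executed.
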(event `ChangeFaColor` :!signature `self.FaColor`
  (params (Color :type "Vector Structure"))
  ;[0.0773 0.744 0] 生成角色3DUI的RT
  (`MeshComponent.SetVectorParameterValueOnMaterials` (`self.Mesh`) "Color" Color)
  (set `self.ToufaColor` Color))

(event `self.ReceiveBeginPlay`)

(event `Key|O`
  (params (Key :type "Key Structure"))
  (bind _returnvalue (`GameplayStatics.GetPlayerController` 0))
  ;[0 0.4155 0.4058] 生成UI
  (:`Pressed`
    (`/Engine/EditorBlueprintResources/StandardMacros.IsValid` (`self.PlayerUI`)
      (:`Is Valid`
        _)
      (:`Is Not Valid`
        (bind _returnvalue_2 (`|CreateWidget` "/Game/UMG/PlayerUMG.PlayerUMG_C"))
        (set `self.PlayerUI` _returnvalue_2)))
    (`UserWidget.AddToViewport` (`self.PlayerUI`) 0)
    (`WidgetBlueprintLibrary.SetInputMode_UIOnlyEx` _returnvalue null)
    (set `PlayerController.bShowMouseCursor` true _returnvalue)
    (`ActorComponent.SetActive` (`self.CharacterMovement`) false false)))

(event `self.ReceiveTick`
  (params (DeltaSeconds :type "Float (single-precision)"))
  (bind (_returnvalue_roll _returnvalue_pitch _returnvalue_yaw) (`KismetMathLibrary.BreakRotator` (`self.GetControlRotation`)))
  (bind _springarm (`self.SpringArm`))
  (bind (_returnvalue_roll_2 _returnvalue_pitch_2) (`KismetMathLibrary.BreakRotator` (`SceneComponent.K2_GetComponentRotation` _springarm)))
  ;[0 0.6087 0.2126] 燃烧草地RT
  (`SceneComponent.K2_SetWorldRotation` _springarm (`KismetMathLibrary.MakeRotator` _returnvalue_roll_2 _returnvalue_pitch_2 _returnvalue_yaw) false false)
  (if (`self.FireRun`)
    (`self.Draw`)))

(event `Key|C`
  (params (Key :type "Key Structure"))
  ;[0.8116 0 0.009777] 清除燃烧
  (:`Pressed`
    (`self.Clear`)))

(event `Key|F`
  (params (Key :type "Key Structure"))
  (bind _fire (`self.Fire`))
  ;[0 0.6087 0.2126] 燃烧草地RT
  (:`Pressed`
    (`/Engine/EditorBlueprintResources/StandardMacros.FlipFlop`
      (:`A`
        (`SceneComponent.SetVisibility` _fire true false)
        (set `self.FireRun` true))
      (:`B`
        (`SceneComponent.SetVisibility` _fire false false)
        (set `self.FireRun` false)))))

(event `Clear`
  ;[0.8116 0 0.009777] 清除燃烧
  (`KismetRenderingLibrary.ClearRenderTarget2D` "/Game/Character/ShiYi/SuperMat/RT.RT"))

(event `Draw`
  (bind _brush_idm (`self.Brush_IDM`))
  (bind _brush_idm_2 (`self.Brush_IDM`))
  ;[0 0.6087 0.2126] 燃烧草地RT
  (`MaterialInstanceDynamic.SetVectorParameterValue` _brush_idm_2 "Position" (`KismetMathLibrary.Conv_VectorToLinearColor` (/ (`self.K2_GetActorLocation`) (`self.MapSize`))))
  (`MaterialInstanceDynamic.SetScalarParameterValue` _brush_idm_2 "Size" (/ (`self.BrushSize`) (`self.MapSize`)))
  (`MaterialInstanceDynamic.SetScalarParameterValue` _brush_idm "Strength" (* (`GameplayStatics.GetWorldDeltaSeconds`) 7.5))
  (`KismetRenderingLibrary.DrawMaterialToRenderTarget` "/Game/Character/ShiYi/SuperMat/RT.RT" _brush_idm))

(event `InputAxis|Camerago`
  (params (AxisValue :type "Float (single-precision)"))
  ;[0 0.773 0.04831] 镜头滚轮
  (bind _output_get (set `self.相机远近` (+ (`self.相机远近`) (* AxisValue 50.0))))
  (if (>= _output_get -50.0)
    (bind _returnvalue (<= _output_get 500.0))
    (if _returnvalue
      (set `SpringArmComponent.TargetArmLength` (`self.相机远近`) (`self.SpringArm`))
      (else
        (set `self.相机远近` 499.0)))
    (else
      (if _returnvalue
        _
        (else
          _))
      (set `self.相机远近` -49.0))))

(event `Key|H`
  (params (Key :type "Key Structure"))
  (bind _mesh (`self.Mesh`))
  (bind _mesh_2 (`self.Mesh`))
  ;[0 0.2126 0.6087] 隐身
  (:`Pressed`
    (`PrimitiveComponent.SetMaterial` _mesh_2 0 "/Game/Character/ShiYi/Tex/yi_Test_Inst.yi_Test_Inst")
    (`PrimitiveComponent.SetMaterial` _mesh_2 1 "/Game/Character/ShiYi/Tex/jia_Test_Inst.jia_Test_Inst")
    (`PrimitiveComponent.SetMaterial` _mesh_2 2 "/Game/Character/ShiYi/Tex/fa_Test_Inst.fa_Test_Inst")
    (`|ExecutionSequence`
      (:`then_0`
        (bind (_direction _newtrack_0) (`Timeline|yinshen` :!via `PlayFromStart` :!label _label)
          (:`Update`
            (`MeshComponent.SetScalarParameterValueOnMaterials` (`self.Mesh`) "Alpha" _newtrack_0))
          (:`Finished`
            (`KismetSystemLibrary.Delay` 6.0)
            (goto _label :!via `ReverseFromEnd`))))
      (:`then_1`
        (`KismetSystemLibrary.Delay` 10.0)
        (`PrimitiveComponent.SetMaterial` _mesh 0 "/Game/Character/ShiYi/Tex/19_-_Default.19_-_Default")
        (`PrimitiveComponent.SetMaterial` _mesh 1 "/Game/Character/ShiYi/Tex/02_-_Default.02_-_Default")
        (`PrimitiveComponent.SetMaterial` _mesh 2 "/Game/Character/ShiYi/Tex/13_-_Default.13_-_Default")
        (goto _label :!via `Stop`)))))

(event `InputAxis|LookRight`
  (params (AxisValue :type "Float (single-precision)"))
  ;[0.1353 0 0.6942] 移动
  (`self.AddControllerYawInput` AxisValue))

(event `Key|K`
  (params (Key :type "Key Structure"))
  ;[0 0.5604 0.2609] 镜头缩进
  (:`Pressed`
    (bind (_direction _zoom) (`Timeline|Time` :!label _label_2)
      (:`Update`
        (`CameraComponent.SetFieldOfView` (`self.Camera`) _zoom))))
  (:`Released`
    (goto _label_2 :!via `Reverse`)))

(event `InputAxis|LookUp`
  (params (AxisValue :type "Float (single-precision)"))
  ;[0.1353 0 0.6942] 移动
  (`SceneComponent.K2_AddRelativeRotation` (`self.SpringArm`) (`KismetMathLibrary.MakeRotator` 0.0 (* AxisValue -1.0)) false false))

(event `InputAxis|MoveForward`
  (params (AxisValue :type "Float (single-precision)"))
  ;[0.1353 0 0.6942] 移动
  (set `self.ForwardInput` AxisValue))

(event `InputAction|Crouch`
  (params (Key :type "Key Structure"))
  ;[0.5797 0 0.2444] 下蹲奔跑
  (:`Pressed`
    (`self.Crouch`))
  (:`Released`
    (`self.UnCrouch`)))

(event `InputAxis|MoveRight`
  (params (AxisValue :type "Float (single-precision)"))
  ;[0.1353 0 0.6942] 移动
  (set `self.RightInput` AxisValue))

(event `InputAction|Attack`
  (params (Key :type "Key Structure"))
  ;[0.3382 0 0.4889] 攻击
  (:`Pressed`
    (set `self.Attack` true))
  (:`Released`
    (set `self.Attack` false)))

(event `InputAction|SpeedUp`
  (params (Key :type "Key Structure"))
  ;[0.5797 0 0.2444] 下蹲奔跑
  (:`Pressed`
    (set `self.IsInRunMode` true))
  (:`Released`
    (set `self.IsInRunMode` false)))

(event `BBB_1`
  (params (CCC :type Boolean))
  ;[0 0.7827 0.03865] 接口
  (if CCC
    (`KismetSystemLibrary.PrintString` "接口测试成功")
    (else
      (`KismetSystemLibrary.PrintString` "接口测试没失败"))))

(fn `UserConstructionScript`
  (bind _returnvalue (`KismetMaterialLibrary.CreateDynamicMaterialInstance` "/Game/Character/ShiYi/SuperMat/Mat_Brush.Mat_Brush"))
  (set `self.Brush_IDM` _returnvalue))